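; DronePawn is an AI drone that patrols linked PatrolPoint actors, pausing briefly at each before moving to the next.
; When an FPS_Character enters its detection sphere, the character becomes its goal and the drone moves toward it.
; Tick smoothly rotates the drone to face the current goal.
; A character entering the explosion sphere triggers Explode, which plays sound and particle effects and destroys the drone.
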(event OnComponentBeginOverlap(Sphere)
  (params (OverlappedComponent :type Primitive%20Component%20Object%20Reference) (OtherActor :type Actor%20Object%20Reference) (OtherComp :type Primitive%20Component%20Object%20Reference) (OtherBodyIndex :type Integer) (bFromSweep :type Boolean) (SweepResult :type Hit%20Result%20Structure%20%28by%20ref%29))
  (bind _asfps_character (Utilities|Casting|CastToFPS_Character OtherActor))
  (bind _output_get (Variables|Default|SetGoalActor _asfps_character))
  (AI|AIMoveTo self "0, 0, 0" _output_get 25.0 false))

(event OnComponentBeginOverlap(ExplodeSphere)
  (params (OverlappedComponent :type Primitive%20Component%20Object%20Reference) (OtherActor :type Actor%20Object%20Reference) (OtherComp :type Primitive%20Component%20Object%20Reference) (OtherBodyIndex :type Integer) (bFromSweep :type Boolean) (SweepResult :type Hit%20Result%20Structure%20%28by%20ref%29))
  (Utilities|Casting|CastToFPS_Character OtherActor)
  (CallFunction|Explode))

(event Collision|EventActorBeginOverlap
  (params (OtherActor :type Actor%20Object%20Reference)))

(event EventTick
  (params (DeltaSeconds :type Float%20%28single-precision%29))
  (bind _goalactor (Variables|Default|GetGoalActor))
  (Utilities|IsValid _goalactor
    (:Is%20Valid
      (Transformation|SetActorRotation (Math|Interpolation|RInterpTo (Transformation|GetActorRotation) (Math|Rotator|FindLookatRotation (Transformation|GetActorLocation) (Transformation|GetActorLocation _goalactor)) DeltaSeconds 5.0)))))

(event EventBeginPlay
  (Utilities|IsValid (Variables|Default|GetGoalActor) :!label _label
    (:Is%20Valid
      (AI|AIMoveTo (AI|GetAIController self) "0, 0, 0" (Variables|Default|GetGoalActor) 25.0 "Disable" "Default" true true
        (:OnMoveFinished
          (bind _aspatrol_point (Utilities|Casting|CastToPatrolPoint (Variables|Default|GetGoalActor)))
          (Variables|Default|SetGoalActor (Variables|/Game/Blueprints/Drone/PatrolPoint.PatrolPoint_C|GetNextPoint _aspatrol_point))
          (Utilities|FlowControl|Delay 1.0)
          (goto _label))))))

(fn ConstructionScript)

(fn Explode
  (Audio|PlaySoundatLocation "/Game/StarterContent/Audio/Explosion_Cue.Explosion_Cue" (Transformation|GetActorLocation) "0, 0, 0" 1.0 1.0 0.0 0 0 0 0)
  (Effects|SpawnEmitteratLocation "/Game/StarterContent/Particles/P_Explosion.P_Explosion" (Transformation|GetActorLocation))
  (Actor|DestroyActor))